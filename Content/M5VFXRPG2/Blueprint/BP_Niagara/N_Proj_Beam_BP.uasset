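; Continuous Niagara beam actor for the player character, with muzzle, beam, impact and beam-end effects.
; Proj_PT_Set assigns the effect assets and attaches the actor to the character.
; Each tick it reads aim data from ThirdPersonCharacter_Fix, drives the beam's Start and End parameters, and shows impact or beam-end effects depending on whether something is targeted.
; When the character's BeamContinue turns false, it deactivates the effects and destroys itself after a delay.
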(event Custom|Proj_PT_Set
  (params (ProjectileFire_PT :type Niagara%20System%20Object%20Reference) (projectile_PT :type Niagara%20System%20Object%20Reference) (ProjectileExplosion_PT :type Niagara%20System%20Object%20Reference) (ProjectileBeamEnd_PT :type Niagara%20System%20Object%20Reference) (TargetPoint :type Vector) (IsTargetObject :type Boolean) (NoneTargetPoint :type Vector) (beamContinue :type Boolean))
  (bind _n_projfire_pt (Variables|Default|GetN_ProjFire_PT))
  (bind _n_projexp_pt (Variables|Default|GetN_ProjExp_PT))
  (bind _n_proj_pt (Variables|Default|GetN_Proj_PT))
  (bind _n_proj_pt_2 (Variables|Default|GetN_Proj_PT))
  ;[1 1 1] Projectile Particle
  (bind _output_get (Variables|Default|Setbeamcontinue beamContinue))
  (if _output_get
    (Variables|Default|SetTargetLocation TargetPoint)
    (else
      (Variables|Default|SetTargetLocation NoneTargetPoint)))
  (Class|NiagaraComponent|SetAsset _n_projfire_pt ProjectileFire_PT true)
  (Components|Activation|SetActive _n_projfire_pt true false)
  (Components|Activation|SetActive _n_projexp_pt false false)
  (Class|NiagaraComponent|SetAsset (Variables|Default|GetN_ProBeamEnd_PT) ProjectileBeamEnd_PT true)
  (Class|NiagaraComponent|SetAsset _n_projexp_pt ProjectileExplosion_PT true)
  (bind _asthird_person_character_fix (Utilities|Casting|CastToThirdPersonCharacter_Fix (Game|GetPlayerCharacter 0)))
  (Transformation|AttachActorToActor self (Components|GetOwner (Variables|/Game/M5VFXRPG2/Blueprint/ThirdPersonCharacter_Fix.ThirdPersonCharacter_Fix_C|GetArrow1 _asthird_person_character_fix)) "None" "KeepWorld" "KeepWorld" "KeepWorld" true)
  (Class|NiagaraComponent|SetAsset _n_proj_pt projectile_PT true)
  (Components|Activation|SetActive _n_proj_pt true false)
  (Class|NiagaraComponent|SetVariablePosition _n_proj_pt_2 "Start" (Variables|Default|GetSourceLocation))
  (Class|NiagaraComponent|SetVariablePosition _n_proj_pt_2 "End" (Variables|Default|GetTargetLocation))
  (if (Variables|Default|Getbeamcontinue)
    _
    (else
      _))
  (Actor|SetLifeSpan 0.0))

(event EventTick
  (params (DeltaSeconds :type Float%20%28single-precision%29))
  (bind _returnvalue (Transformation|GetActorLocation))
  (bind _n_proj_pt (Variables|Default|GetN_Proj_PT))
  (bind _n_projexp_pt (Variables|Default|GetN_ProjExp_PT))
  (bind _n_probeamend_pt (Variables|Default|GetN_ProBeamEnd_PT))
  ;[1 1 1] Continuous Beam
  (bind _asthird_person_character_fix (Utilities|Casting|CastToThirdPersonCharacter_Fix (Game|GetPlayerCharacter 0)))
  (Variables|Default|SetTargetLocation (Variables|/Game/M5VFXRPG2/Blueprint/ThirdPersonCharacter_Fix.ThirdPersonCharacter_Fix_C|GetTargetHitLocation _asthird_person_character_fix))
  (Variables|Default|SetSourceLocation (Transformation|GetWorldLocation (Variables|/Game/M5VFXRPG2/Blueprint/ThirdPersonCharacter_Fix.ThirdPersonCharacter_Fix_C|GetArrow1 _asthird_person_character_fix)))
  (Variables|Default|SetImpactnormal (Math|Conversions|RotationFromXVector (Variables|/Game/M5VFXRPG2/Blueprint/ThirdPersonCharacter_Fix.ThirdPersonCharacter_Fix_C|GetImpactnormal _asthird_person_character_fix)))
  (Transformation|SetWorldRotation (Variables|Default|GetN_ProjFire_PT) (Transformation|GetWorldRotation (Variables|/Game/M5VFXRPG2/Blueprint/ThirdPersonCharacter_Fix.ThirdPersonCharacter_Fix_C|GetArrow1 _asthird_person_character_fix)) false false)
  (Transformation|SetWorldRotation (Variables|Default|GetSphere) (Math|Rotator|FindLookatRotation _returnvalue (+ _returnvalue "0, 0, 0")) false false)
  (bind _asthird_person_character_fix_2 (Utilities|Casting|CastToThirdPersonCharacter_Fix (Game|GetPlayerCharacter 0)))
  (bind _output_get (Variables|Default|Setbeamcontinue (Variables|/Game/M5VFXRPG2/Blueprint/ThirdPersonCharacter_Fix.ThirdPersonCharacter_Fix_C|GetbeamContinue _asthird_person_character_fix_2)))
  (if _output_get
    (Class|NiagaraComponent|SetVariablePosition _n_proj_pt "Start" (Variables|Default|GetSourceLocation))
    (Class|NiagaraComponent|SetVariablePosition _n_proj_pt "End" (Variables|Default|GetTargetLocation))
    (if (Variables|/Game/M5VFXRPG2/Blueprint/ThirdPersonCharacter_Fix.ThirdPersonCharacter_Fix_C|GetTargeted _asthird_person_character_fix_2)
      (Components|Activation|SetActive _n_projexp_pt true false)
      (Transformation|SetWorldRotation _n_projexp_pt (Variables|Default|GetImpactnormal) false false)
      (Transformation|SetWorldLocation _n_projexp_pt (Variables|Default|GetTargetLocation) false false)
      (Utilities|FlowControl|Delay 0.0)
      (Components|Activation|SetActive (Variables|Default|GetN_ProBeamEnd_PT) false false)
      (else
        (Components|Activation|SetActive _n_probeamend_pt true false)
        (Utilities|FlowControl|Sequence
          (:then_0
            (Transformation|SetWorldLocation _n_probeamend_pt (Variables|Default|GetTargetLocation) false false)
            (Utilities|FlowControl|Delay 0.0)
            (Components|Activation|SetActive (Variables|Default|GetN_ProjExp_PT) false false))
          (:then_1
            (Utilities|FlowControl|Delay 0.5)
            (Development|PrintString "none Target" true true "(R=1.000000,G=0.000000,B=0.000000,A=1.000000)" 0.5)))))
    (else
      (Components|Activation|SetActive (Variables|Default|GetN_Proj_PT) false false)
      (Actor|SetLifeSpan 2.0)
      (Components|Activation|SetActive (Variables|Default|GetN_Proj_PT) false false)
      (Utilities|FlowControl|Delay 2.0)
      (Actor|DestroyActor))))

(fn ConstructionScript)