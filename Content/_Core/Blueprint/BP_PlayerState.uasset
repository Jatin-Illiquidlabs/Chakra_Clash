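; Player state for a networked, move-based combat game, holding health, death, player type, index, selected move and charge.
; Authority checks route changes through server and client event pairs.
; Each move locks selection and adjusts charge by type, though only the client event applies the passed move; the others use Charge.
; Damage updates health and death, and UpdateStatsInGameState clears the lock and pushes stats to GS_GameStateBase.
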(event Custom|Update%20Current%20Move%20Server
  (params (CurrentMove :type E_MoveType%20Enum :default "NewEnumerator1"))
  (Variables|Default|SetCurrentMove CurrentMove))

(event Custom|Update%20Health%20Server
  (params (Health :type Integer) (IsDead :type Boolean))
  (Variables|Default|SetPlayerHealth Health)
  (Variables|Default|SetIsDead IsDead))

(event Custom|SetPlayerIndex
  (params (PlayerIndex :type Integer))
  (Networking|SwitchHasAuthority
    (:Authority
      (CallFunction|SetPlayerIndexClient PlayerIndex))
    (:Remote
      (CallFunction|SetPlayerIndexServer PlayerIndex))))

(event Custom|SetPlayerIndex_Server
  (params (PlayerIndex :type Integer))
  (CallFunction|SetPlayerIndexClient PlayerIndex)
  (Variables|Default|SetPlayerIndex PlayerIndex))

(event Custom|UpdateHealth
  (params (Damage :type Integer) (PlayerNum :type Integer))
  (if (== PlayerNum (Variables|Default|GetPlayerNum))
    (Variables|Default|SetPlayerHealth (- (Variables|Default|GetPlayerHealth) Damage))
    (if (<= (Variables|Default|GetPlayerHealth) 0)
      (Variables|Default|SetIsDead true))
    (Networking|SwitchHasAuthority
      (:Remote
        (CallFunction|UpdateHealthServer (Variables|Default|GetPlayerHealth) (Variables|Default|GetIsDead))))))

(event Custom|SetPlayerIndex_Client
  (params (PlayerIndex :type Integer))
  (Variables|Default|SetPlayerIndex PlayerIndex))

(event Custom|Set%20Current%20Move
  (params (New%20Move :type E_MoveType%20Enum :default "NewEnumerator1"))
  (Networking|SwitchHasAuthority
    (:Authority
      (CallFunction|SetCurrentMoveinClients New%20Move))
    (:Remote
      (CallFunction|SetCurrentMoveinServer "NewEnumerator1")))
  (if (not (Variables|Default|GetHasSelectedMove))
    (Variables|Default|SetHasSelectedMove true)
    (bind _output_get (Variables|Default|SetCurrentMove "NewEnumerator1"))
    (switch Utilities|FlowControl|Switch|SwitchonE_MoveType _output_get
      (:NewEnumerator1
        (Variables|Default|SetChargeChange 1))
      (:NewEnumerator2
        (Variables|Default|SetChargeChange -1))
      (:NewEnumerator3
        (Variables|Default|SetChargeChange -2))
      (:NewEnumerator4
        (Variables|Default|SetChargeChange -3))
      (:NewEnumerator6
        (Variables|Default|SetChargeChange 0)))
    (Variables|Default|SetCurrentCharge (+ (Variables|Default|GetCurrentCharge) (Variables|Default|GetChargeChange)))))

(event Custom|UpdatePlayerType
  (params (SelectedPlayerType :type PlayerType%20Enum :default "Deva"))
  (Networking|SwitchHasAuthority
    (:Authority
      (CallFunction|UpdatePlayerTypeinServer SelectedPlayerType))
    (:Remote
      (CallFunction|UpdatePlayerTypeinClient SelectedPlayerType))))

(event Custom|UpdateStatsInGameState
  (Variables|Default|SetHasSelectedMove false)
  (Networking|SwitchHasAuthority
    (:Authority
      (bind _asgs_game_state_base (Utilities|Casting|CastToGS_GameStateBase (Game|GetGameState)))
      (Default|UpdateStatsinClients _asgs_game_state_base (Variables|Default|GetSelectedPlayerType) (Variables|Default|GetPlayerHealth) (Variables|Default|GetCurrentCharge)))
    (:Remote
      (bind _asgs_game_state_base_2 (Utilities|Casting|CastToGS_GameStateBase (Game|GetGameState)))
      (Default|UpdateStatsinServer _asgs_game_state_base_2 (Variables|Default|GetSelectedPlayerType) (Variables|Default|GetPlayerHealth) (Variables|Default|GetCurrentCharge)))))

(event Custom|SetCurrentMoveInClients
  (params (NewMove :type E_MoveType%20Enum :default "NewEnumerator1"))
  (if (not (Variables|Default|GetHasSelectedMove))
    (Variables|Default|SetHasSelectedMove true)
    (bind _output_get (Variables|Default|SetCurrentMove NewMove))
    (switch Utilities|FlowControl|Switch|SwitchonE_MoveType _output_get
      (:NewEnumerator1
        (Variables|Default|SetChargeChange 1))
      (:NewEnumerator2
        (Variables|Default|SetChargeChange -1))
      (:NewEnumerator3
        (Variables|Default|SetChargeChange -2))
      (:NewEnumerator4
        (Variables|Default|SetChargeChange -3))
      (:NewEnumerator6
        (Variables|Default|SetChargeChange 0)))
    (Variables|Default|SetCurrentCharge (+ (Variables|Default|GetCurrentCharge) (Variables|Default|GetChargeChange)))))

(event Custom|SetCurrentMoveInServer
  (params (NewMove :type E_MoveType%20Enum :default "NewEnumerator1"))
  (CallFunction|SetCurrentMoveinClients NewMove)
  (if (not (Variables|Default|GetHasSelectedMove))
    (Variables|Default|SetHasSelectedMove true)
    (bind _output_get (Variables|Default|SetCurrentMove "NewEnumerator1"))
    (switch Utilities|FlowControl|Switch|SwitchonE_MoveType _output_get
      (:NewEnumerator1
        (Variables|Default|SetChargeChange 1))
      (:NewEnumerator2
        (Variables|Default|SetChargeChange -1))
      (:NewEnumerator3
        (Variables|Default|SetChargeChange -2))
      (:NewEnumerator4
        (Variables|Default|SetChargeChange -3))
      (:NewEnumerator6
        (Variables|Default|SetChargeChange 0)))
    (Variables|Default|SetCurrentCharge (+ (Variables|Default|GetCurrentCharge) (Variables|Default|GetChargeChange)))))

(event Custom|UpdatePlayerTypeInClient
  (params (SelectedPlayerType :type PlayerType%20Enum :default "Deva"))
  (Variables|Default|SetSelectedPlayerType SelectedPlayerType))

(event Custom|UpdatePlayerTypeInServer
  (params (SelectedPlayerType :type PlayerType%20Enum :default "Deva"))
  (CallFunction|UpdatePlayerTypeinClient SelectedPlayerType))

(event EventBeginPlay
  (Variables|Default|SetIsDead false))

(event EventTick
  (params (DeltaSeconds :type Float%20%28single-precision%29)))

(fn ConstructionScript)