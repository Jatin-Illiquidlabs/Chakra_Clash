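; Base player character for a two-player, simultaneous-move duel between Deva and Shakti, built on charge, attack and evade moves.
; SetCurrentMove stores the choice in BP_PlayerState, adjusts local charge and evades, and forwards it to the server from remote instances.
; PlayMove resolves move pairs through a nested branch chain, playing Level Sequences and updating GI_Game health and charge.
; It also registers with the HUD and shows the game-over screen.
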(event Custom|GameOver
  (if (Pawn|IsLocallyControlled)
    (bind _returnvalue (UserInterface|CreateWidget "/Game/_Core/UI_FrameWork/Widgets/GameOver_Screen.GameOver_Screen_C" (Game|GetPlayerController 0)))
    (UserInterface|Viewport|AddtoViewport _returnvalue 0)
    (CallFunction|GameOverServer)))

(event Custom|UpdateHealth
  (params (Damage :type Integer) (PlayerNum :type Integer))
  (bind _asgi_game (Utilities|Casting|CastToGI_Game (Game|GetGameInstance)))
  (switch int PlayerNum
    (:0
      (Default|UpdateDevaHealth _asgi_game Damage))
    (:1
      (Default|UpdateShaktiHealth _asgi_game Damage))))

(event Custom|SetPlayerRotation
  (params (NewRotation :type Rotator%20%28by%20ref%29))
  (Pawn|SetControlRotation (Game|GetPlayerController 0) NewRotation))

(event Custom|GameOverServer
  (bind _returnvalue (UserInterface|CreateWidget "/Game/_Core/UI_FrameWork/Widgets/GameOver_Screen.GameOver_Screen_C" (Game|GetPlayerController 0)))
  (UserInterface|Viewport|AddtoViewport _returnvalue 0))

(event Custom|UpdateMoveInServer
  (params (CurrentMove :type E_MoveType%20Enum :default "NewEnumerator1"))
  (Variables|Default|SetCurrentMove CurrentMove))

(event Custom|UpdateCharge
  (params (PlayerNum :type Integer) (ChangeAmount :type Integer))
  (bind _asgi_game (Utilities|Casting|CastToGI_Game (Game|GetGameInstance)))
  (switch int PlayerNum
    (:0
      (Default|UpdateDevaCharge _asgi_game ChangeAmount))
    (:1
      (Default|UpdateShaktiCharge _asgi_game ChangeAmount))))

(event EventBeginPlay
  (if (Pawn|IsLocallyControlled)
    (bind _asgame_hud (Utilities|Casting|CastToGame_HUD (HUD|GetHUD (Game|GetPlayerController 0)))
      (:then
        (Development|PrintString "Game HUD")
        (Variables|/Game/_Core/UI_FrameWork/Widgets/Menus/Game_HUD_Screen_2.Game_HUD_Screen_2_C|SetPlayer%20Pawn (Variables|/Game/_Core/UI_FrameWork/UI_Stuff/Game_HUD.Game_HUD_C|GetGame%20HUD _asgame_hud) self)
        (bind _asgi_game (Utilities|Casting|CastToGI_Game (Game|GetGameInstance))))
      (:CastFailed
        (Development|PrintString "Could not cast to game Hud")))))

(fn ConstructionScript)

(fn SetCurrentMove
  (params (NewMove :type E_MoveType%20Enum :default "NewEnumerator1"))
  (bind _asbp_player_state (Utilities|Casting|CastToBP_PlayerState (Variables|GetPlayerState)))
  (Variables|/Game/_Core/Blueprint/BP_PlayerState.BP_PlayerState_C|SetCurrentMove _asbp_player_state NewMove)
  (bind _output_get (Variables|Default|SetCurrentMove NewMove))
  (switch Utilities|FlowControl|Switch|SwitchonE_MoveType _output_get
    (:NewEnumerator1
      (LocalVariables|SetChargeChange 1)
      (Variables|Default|SetEvadesLeft 2 :!label _label))
    (:NewEnumerator2
      (LocalVariables|SetChargeChange -1)
      (goto _label))
    (:NewEnumerator3
      (LocalVariables|SetChargeChange -2)
      (goto _label))
    (:NewEnumerator4
      (LocalVariables|SetChargeChange -3)
      (goto _label))
    (:NewEnumerator6
      (LocalVariables|SetChargeChange 0)))
  (Variables|Default|SetCurrentCharge (+ (Variables|Default|GetCurrentCharge) (LocalVariables|GetChargeChange)))
  (Networking|SwitchHasAuthority
    (:Remote
      (bind _asbp_player_state_2 (Utilities|Casting|CastToBP_PlayerState (Variables|GetPlayerState)))
      (Default|UpdateCurrentMoveServer _asbp_player_state_2 NewMove))))

(fn ResetCurrentMove
  (Utilities|FlowControl|Sequence
    (:then_0
      (CallFunction|SetCurrentMove "NewEnumerator1")
      (bind _asgm_game (Utilities|Casting|CastToGM_Game (Game|GetGameMode)))
      (Default|StartCountdown _asgm_game))
    (:then_1
      (switch Utilities|FlowControl|Switch|SwitchonE_MoveType (Variables|Default|GetCurrentMove)
        (:NewEnumerator5
          _)
        (:NewEnumerator6
          _))
      (Variables|Default|SetEvadesLeft (- (Variables|Default|GetEvadesLeft) 1)))))

(fn PlayMove
  (params (DevaMove :type E_MoveType%20Enum :default "NewEnumerator1") (ShaktiMove :type E_MoveType%20Enum :default "NewEnumerator1"))
  (if (and (Utilities|Enum|Equal(Enum) DevaMove "NewEnumerator1") (Utilities|Enum|Equal(Enum) ShaktiMove "NewEnumerator1"))
    (CallFunction|PlaySequence (Variables|Sequences|GetDevaChargeShaktiCharge))
    (CallFunction|UpdateCharge 0 1)
    (CallFunction|UpdateCharge 1 1)
    (elif (and (Utilities|Enum|Equal(Enum) DevaMove "NewEnumerator2") (Utilities|Enum|Equal(Enum) ShaktiMove "NewEnumerator1"))
      (CallFunction|PlaySequence (Variables|Sequences|GetDevaAttack1ShaktiCharge))
      (CallFunction|UpdateHealth 1 1)
      (CallFunction|UpdateCharge 0 -1)
      (CallFunction|UpdateCharge 1 1)
      (elif (and (Utilities|Enum|Equal(Enum) DevaMove "NewEnumerator3") (Utilities|Enum|Equal(Enum) ShaktiMove "NewEnumerator1"))
        (CallFunction|PlaySequence (Variables|Sequences|GetDevaAttack2ShaktiCharge))
        (CallFunction|UpdateHealth 2 1)
        (CallFunction|UpdateCharge 0 -2)
        (CallFunction|UpdateCharge 1 1)
        (elif (and (Utilities|Enum|Equal(Enum) DevaMove "NewEnumerator1") (Utilities|Enum|Equal(Enum) ShaktiMove "NewEnumerator2"))
          (CallFunction|PlaySequence (Variables|Sequences|GetShaktiAttack1DevaCharge))
          (CallFunction|UpdateHealth 1)
          (CallFunction|UpdateCharge 1 -1)
          (CallFunction|UpdateCharge 0 1)
          (elif (and (Utilities|Enum|Equal(Enum) DevaMove "NewEnumerator1") (Utilities|Enum|Equal(Enum) ShaktiMove "NewEnumerator3"))
            (CallFunction|PlaySequence (Variables|Sequences|GetShaktiAttack2DevaCharge))
            (CallFunction|UpdateHealth 2)
            (CallFunction|UpdateCharge 1 -2)
            (CallFunction|UpdateCharge 0 1)
            (elif (and (Utilities|Enum|Equal(Enum) DevaMove "NewEnumerator4") (Utilities|Enum|Equal(Enum) ShaktiMove "NewEnumerator1"))
              (CallFunction|PlaySequence (Variables|Sequences|GetDevaNukesShakti))
              (CallFunction|UpdateHealth 3 1)
              (CallFunction|UpdateCharge 0 -3)
              (CallFunction|UpdateCharge 1 1)
              (elif (and (Utilities|Enum|Equal(Enum) DevaMove "NewEnumerator1") (Utilities|Enum|Equal(Enum) ShaktiMove "NewEnumerator4"))
                (CallFunction|PlaySequence (Variables|Sequences|GetShaktiNukesDeva))
                (CallFunction|UpdateHealth 3)
                (CallFunction|UpdateCharge 1 -3)
                (CallFunction|UpdateCharge 0 1)
                (elif (and (Utilities|Enum|Equal(Enum) DevaMove "NewEnumerator2") (Utilities|Enum|Equal(Enum) ShaktiMove "NewEnumerator6"))
                  (CallFunction|PlaySequence (Variables|Sequences|GetDevaAttack1ShaktiEvades))
                  (CallFunction|UpdateCharge 0 -1)
                  (elif (and (Utilities|Enum|Equal(Enum) DevaMove "NewEnumerator3") (Utilities|Enum|Equal(Enum) ShaktiMove "NewEnumerator6"))
                    (CallFunction|PlaySequence (Variables|Sequences|GetDevaAttack2ShaktiEvades))
                    (CallFunction|UpdateCharge 0 -2)
                    (elif (and (Utilities|Enum|Equal(Enum) DevaMove "NewEnumerator4") (Utilities|Enum|Equal(Enum) ShaktiMove "NewEnumerator6"))
                      (CallFunction|PlaySequence (Variables|Sequences|GetDevaAttack3ShaktiEvades))
                      (CallFunction|UpdateCharge 0 -3)
                      (elif (and (Utilities|Enum|Equal(Enum) DevaMove "NewEnumerator6") (Utilities|Enum|Equal(Enum) ShaktiMove "NewEnumerator2"))
                        (CallFunction|PlaySequence (Variables|Sequences|GetShaktiAttack1DevaEvades))
                        (CallFunction|UpdateCharge 1 -1)
                        (elif (and (Utilities|Enum|Equal(Enum) DevaMove "NewEnumerator6") (Utilities|Enum|Equal(Enum) ShaktiMove "NewEnumerator3"))
                          (CallFunction|PlaySequence (Variables|Sequences|GetShaktiAttack2DevaEvades))
                          (CallFunction|UpdateCharge 1 -2)
                          (elif (and (Utilities|Enum|Equal(Enum) DevaMove "NewEnumerator6") (Utilities|Enum|Equal(Enum) ShaktiMove "NewEnumerator4"))
                            (CallFunction|PlaySequence (Variables|Sequences|GetShaktiAttack3DevaEvades))
                            (CallFunction|UpdateCharge 1 -3)
                            (elif (and (Utilities|Enum|Equal(Enum) DevaMove "NewEnumerator2") (Utilities|Enum|Equal(Enum) ShaktiMove "NewEnumerator2"))
                              (CallFunction|PlaySequence (Variables|Sequences|GetShaktiAttack1DevaAttack1))
                              (CallFunction|UpdateHealth 1)
                              (CallFunction|UpdateHealth 1 1)
                              (CallFunction|UpdateCharge 0 -1)
                              (CallFunction|UpdateCharge 1 -1)
                              (elif (and (Utilities|Enum|Equal(Enum) DevaMove "NewEnumerator3") (Utilities|Enum|Equal(Enum) ShaktiMove "NewEnumerator2"))
                                (CallFunction|PlaySequence (Variables|Sequences|GetShaktiAttack1DevaAttack2))
                                (CallFunction|UpdateHealth 1)
                                (CallFunction|UpdateHealth 2 1)
                                (CallFunction|UpdateCharge 0 -1)
                                (CallFunction|UpdateCharge 1 -2)
                                (elif (and (Utilities|Enum|Equal(Enum) DevaMove "NewEnumerator4") (Utilities|Enum|Equal(Enum) ShaktiMove "NewEnumerator2"))
                                  (CallFunction|PlaySequence (Variables|Sequences|GetShaktiAttack1DevaAttack3))
                                  (CallFunction|UpdateHealth 1)
                                  (CallFunction|UpdateHealth 3 1)
                                  (CallFunction|UpdateCharge 0 -1)
                                  (CallFunction|UpdateCharge 1 -3)
                                  (elif (and (Utilities|Enum|Equal(Enum) DevaMove "NewEnumerator2") (Utilities|Enum|Equal(Enum) ShaktiMove "NewEnumerator3"))
                                    (CallFunction|PlaySequence (Variables|Sequences|GetShaktiAttack2DevaAttack1))
                                    (CallFunction|UpdateHealth 2)
                                    (CallFunction|UpdateHealth 1 1)
                                    (CallFunction|UpdateCharge 0 -2)
                                    (CallFunction|UpdateCharge 1 -1)
                                    (elif (and (Utilities|Enum|Equal(Enum) DevaMove "NewEnumerator3") (Utilities|Enum|Equal(Enum) ShaktiMove "NewEnumerator3"))
                                      (CallFunction|PlaySequence (Variables|Sequences|GetShaktiAttack2DevaAttack2))
                                      (CallFunction|UpdateHealth 2)
                                      (CallFunction|UpdateHealth 2 1)
                                      (CallFunction|UpdateCharge 0 -2)
                                      (CallFunction|UpdateCharge 1 -2)
                                      (elif (and (Utilities|Enum|Equal(Enum) DevaMove "NewEnumerator4") (Utilities|Enum|Equal(Enum) ShaktiMove "NewEnumerator3"))
                                        (CallFunction|PlaySequence (Variables|Sequences|GetShaktiAttack2DevaAttack3))
                                        (CallFunction|UpdateHealth 2)
                                        (CallFunction|UpdateHealth 3 1)
                                        (CallFunction|UpdateCharge 0 -2)
                                        (CallFunction|UpdateCharge 1 -3)
                                        (elif (and (Utilities|Enum|Equal(Enum) DevaMove "NewEnumerator2") (Utilities|Enum|Equal(Enum) ShaktiMove "NewEnumerator4"))
                                          (CallFunction|PlaySequence (Variables|Sequences|GetShaktiAttack3DevaAttack1))
                                          (CallFunction|UpdateHealth 3)
                                          (CallFunction|UpdateHealth 1 1)
                                          (CallFunction|UpdateCharge 0 -3)
                                          (CallFunction|UpdateCharge 1 -1)
                                          (elif (and (Utilities|Enum|Equal(Enum) DevaMove "NewEnumerator3") (Utilities|Enum|Equal(Enum) ShaktiMove "NewEnumerator4"))
                                            (CallFunction|PlaySequence (Variables|Sequences|GetShaktiAttack3DevaAttack2))
                                            (CallFunction|UpdateHealth 3)
                                            (CallFunction|UpdateHealth 2 1)
                                            (CallFunction|UpdateCharge 0 -3)
                                            (CallFunction|UpdateCharge 1 -2)
                                            (elif (and (Utilities|Enum|Equal(Enum) DevaMove "NewEnumerator4") (Utilities|Enum|Equal(Enum) ShaktiMove "NewEnumerator4"))
                                              (CallFunction|PlaySequence (Variables|Sequences|GetShaktiAttack3DevaAttack3))
                                              (CallFunction|UpdateHealth 3)
                                              (CallFunction|UpdateHealth 3 1)
                                              (CallFunction|UpdateCharge 0 -3)
                                              (CallFunction|UpdateCharge 1 -3)
                                              (else
                                                (CallFunction|PlaySequence (Variables|Sequences|GetDevaChargeShaktiCharge))))))))))))))))))))))))))

(fn OnRepCurrentMove)

(fn PlaySequence
  (params (LevelSequence :type Level%20Sequence%20Object%20Reference))
  (bind _outactor (Sequencer|Player|CreateLevelSequencePlayer LevelSequence (Utilities|Struct|MakeMovieSceneSequencePlaybackSettings false "(Value=0)" 1.0 0.0 false true true false false false true false)))
  (Sequencer|Player|Play (Variables|/Script/LevelSequence.LevelSequenceActor|GetSequencePlayer _outactor) :!class /Script/MovieScene.MovieSceneSequencePlayer))