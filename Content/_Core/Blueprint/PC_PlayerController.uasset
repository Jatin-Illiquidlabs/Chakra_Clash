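; Player controller for a networked two-player game with Deva and Shakti, handling player identity, HUD setup and move playback.
; Player index follows the game instance's selected player; index and HUD name updates route by authority through server and client events.
; On possession it caches the BP_BaseCharacter pawn, then forwards both players' moves to it locally and through a server event.
; It also caches the game HUD, shows the cursor and recreates the countdown timer widget.
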(event Custom|ShowCountdown
  (Utilities|IsValid (Variables|Default|GetTimerWidget)
    (:Is%20Valid
      (Widget|RemovefromParent (Variables|Default|GetTimerWidget)))
    (:Is%20Not%20Valid
      _))
  (bind _returnvalue (UserInterface|CreateWidget "/Game/_Core/Widgets/WBP_Timer.WBP_Timer_C"))
  (UserInterface|Viewport|AddtoViewport _returnvalue 0)
  (Variables|Default|SetTimerWidget _returnvalue))

(event Custom|PlayMoveServer
  (params (DevaMove :type E_MoveType%20Enum :default "NewEnumerator1") (ShaktiMove :type E_MoveType%20Enum :default "NewEnumerator1"))
  (Default|PlayMove (Variables|Default|GetPossessed%20Pawn) DevaMove ShaktiMove))

(event Custom|PlayMove
  (params (DevaMove :type E_MoveType%20Enum :default "NewEnumerator1") (ShaktiMove :type E_MoveType%20Enum :default "NewEnumerator1"))
  (Default|PlayMove (Variables|Default|GetPossessed%20Pawn) DevaMove ShaktiMove)
  (CallFunction|PlayMoveServer DevaMove ShaktiMove))

(event Custom|StartGsme
  (Variables|Default|SetbShowMouseCursor true)
  (bind _asgame_hud (Utilities|Casting|CastToGame_HUD (HUD|GetHUD)))
  (Variables|Default|SetAs%20Game%20HUD _asgame_hud))

(event Custom|SetPlayerIndex_Server
  (CallFunction|SetPlayerIndexClients)
  (bind _asgi_game (Utilities|Casting|CastToGI_Game (Game|GetGameInstance)))
  (switch Utilities|FlowControl|Switch|SwitchonPlayerType (Variables|/Script/chakra_clash.EOSGameInstance|GetSelectedPlayer _asgi_game)
    (:Deva
      (Variables|Default|SetPlayerIndex 0))
    (:Shakti
      (Variables|Default|SetPlayerIndex 1))))

(event Custom|SetPlayerIndex_Clients
  (bind _asgi_game (Utilities|Casting|CastToGI_Game (Game|GetGameInstance)))
  (switch Utilities|FlowControl|Switch|SwitchonPlayerType (Variables|/Script/chakra_clash.EOSGameInstance|GetSelectedPlayer _asgi_game)
    (:Deva
      (Variables|Default|SetPlayerIndex 0))
    (:Shakti
      (Variables|Default|SetPlayerIndex 1))))

(event Custom|SetPlayerIndex
  (Networking|SwitchHasAuthority
    (:Authority
      (CallFunction|SetPlayerIndexClients))
    (:Remote
      (CallFunction|SetPlayerIndexServer))))

(event Custom|SetPlayersName
  (Networking|SwitchHasAuthority
    (:Authority
      (CallFunction|SetPlayersNameClient))
    (:Remote
      (CallFunction|SetPlayersNameServer))))

(event Custom|SetPlayersName_Server
  (CallFunction|SetPlayersNameClient)
  (Default|SetPlayersName (Variables|/Game/_Core/UI_FrameWork/UI_Stuff/Game_HUD.Game_HUD_C|GetGame%20HUD (Variables|Default|GetAs%20Game%20HUD)))
  (Development|PrintString "UPDATING NAME ON CLIEENT!!!!!!!!!!!!!!!!!!!!!!!!!!!!!!!!!!!!!!!!!!!!!" true true "(R=0.000000,G=0.660000,B=1.000000,A=1.000000)" 1e+01))

(event Custom|SetPlayersName_Client
  (Default|SetPlayersName (Variables|/Game/_Core/UI_FrameWork/UI_Stuff/Game_HUD.Game_HUD_C|GetGame%20HUD (Variables|Default|GetAs%20Game%20HUD))))

(event EventBeginPlay)

(event EventPossess
  (params (PossessedPawn :type Pawn%20Object%20Reference))
  (bind _asbp_base_character (Utilities|Casting|CastToBP_BaseCharacter PossessedPawn))
  (Variables|Default|SetPossessed%20Pawn _asbp_base_character))

(fn ConstructionScript)

(fn GetSpawnIndex)