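; Game state that holds Health and Charge for two players, Deva and Shakti, and runs a move countdown.
; UpdateStatsInServer forwards stats to UpdateStatsInClients, which stores them by CurrentPlayer; its own switch is fixed to Deva instead of reading CurrentPlayer.
; Count starts a looping one-second timer that decrements TimerCount from five and calls GM_Game's PlayMove at -1, without clearing the timer.
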(event Custom|Count
  (Variables|Default|SetTimerCount 5)
  (Utilities|Time|SetTimerbyEvent (delegate Custom|StartTimer) 1.0 true))

(event Custom|UpdateStatsInServer
  (params (CurrentPlayer :type PlayerType%20Enum :default "Deva") (Health :type Integer) (Charge :type Integer))
  (CallFunction|UpdateStatsinClients CurrentPlayer Health Charge)
  (switch Utilities|FlowControl|Switch|SwitchonPlayerType "Deva"
    (:Deva
      (Variables|Default|SetDevaHealth Health)
      (Variables|Default|SetDevaCharge Charge))
    (:Shakti
      (Variables|Default|SetShaktiHealth Health)
      (Variables|Default|SetShaktiCharge Charge))))

(event Custom|UpdateStatsInClients
  (params (CurrentPlayer :type PlayerType%20Enum :default "Deva") (Health :type Integer) (Charge :type Integer))
  (switch Utilities|FlowControl|Switch|SwitchonPlayerType CurrentPlayer
    (:Deva
      (Variables|Default|SetDevaHealth Health)
      (Variables|Default|SetDevaCharge Charge))
    (:Shakti
      (Variables|Default|SetShaktiHealth Health)
      (Variables|Default|SetShaktiCharge Charge))))

(event Custom|StartTimer
  (bind _timercount (Variables|Default|GetTimerCount))
  (Math|Integer|DecrementInt _timercount
    (:%20%20
      (if (== _timercount -1)
        (bind _asgm_game (Utilities|Casting|CastToGM_Game (Game|GetGameMode)))
        (Default|PlayMove _asgm_game)))))

(event EventBeginPlay)

(event EventTick
  (params (DeltaSeconds :type Float%20%28single-precision%29)))

(fn ConstructionScript)