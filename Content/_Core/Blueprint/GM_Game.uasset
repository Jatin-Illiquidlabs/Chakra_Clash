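; Game mode for a two-player, round-based Deva vs Shakti match, handling player spawning, rounds and game over.
; PostLogin spawns and possesses each character at an index-named PlayerStart, giving the second player the opposite slot, then starts the countdown once two join.
; Rounds check GI_Game health for game over or run the GameState countdown.
; PlayMove collects both players' moves and passes them to the host controller.
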(event Custom|Countdown
  ;[0 1 0.8988] CountDown
  (for _array_element (Variables|Default|GetPlayers)
    (Default|ShowCountdown _array_element))
  (Networking|SwitchHasAuthority
    (:Authority
      (bind _asgs_game_state_base (Utilities|Casting|CastToGS_GameStateBase (Game|GetGameState)))
      (Default|Count _asgs_game_state_base))))

(event Custom|PlayMove
  (for _array_element (Variables|Default|GetPlayers)
    (bind _asbp_player_state (Utilities|Casting|CastToBP_PlayerState (Variables|/Script/Engine.Controller|GetPlayerState _array_element)))
    (switch int (Variables|/Game/_Core/Blueprint/BP_BaseCharacter.BP_BaseCharacter_C|GetPlayerNum (Variables|/Game/_Core/Blueprint/PC_PlayerController.PC_PlayerController_C|GetPossessed%20Pawn _array_element)) ; 0: Deva Move\n1: Shakti Move
      (:0
        (Variables|Default|SetDevaMove (Variables|/Game/_Core/Blueprint/BP_PlayerState.BP_PlayerState_C|GetCurrentMove _asbp_player_state))
        (Development|PrintString (Utilities|String|Append "DEVAAAAAAAAAAAAAAA" ":       " (Utilities|String|EnumtoString (Variables|/Game/_Core/Blueprint/BP_PlayerState.BP_PlayerState_C|GetCurrentMove _asbp_player_state))) true true "(R=1.000000,G=0.004636,B=0.000000,A=1.000000)" 5.0))
      (:1
        (Variables|Default|SetShaktiMove (Variables|/Game/_Core/Blueprint/BP_PlayerState.BP_PlayerState_C|GetCurrentMove _asbp_player_state))
        (Development|PrintString (Utilities|String|Append "SHAKTIiiiiiiiiiiiiiii" ":       " (Utilities|String|EnumtoString (Variables|/Game/_Core/Blueprint/BP_PlayerState.BP_PlayerState_C|GetCurrentMove _asbp_player_state))) true true "(R=0.000000,G=0.660000,B=1.000000,A=1.000000)" 5.0))))
  (Default|PlayMove (Variables|Default|GetHostPlayer) (Variables|Default|GetDevaMove) (Variables|Default|GetShaktiMove))
  (Utilities|FlowControl|Delay 1.0)
  (for _array_element_2 (Variables|Default|GetPlayers)
    (Default|ResetCurrentMove (Variables|/Game/_Core/Blueprint/PC_PlayerController.PC_PlayerController_C|GetPossessed%20Pawn _array_element_2))))

(event Custom|StartCountdown
  ;[0 1 0.8988] CountDown
  (if (Variables|Default|GetRoundStarted)
    (Utilities|FlowControl|Delay 5.0)
    (else
      (Variables|Default|SetRoundStarted true)))
  (bind _asgi_game (Utilities|Casting|CastToGI_Game (Game|GetGameInstance)))
  (if (or (<= (Variables|/Game/_Core/Blueprint/GI_Game.GI_Game_C|GetDevaHealth _asgi_game) 0) (<= (Variables|/Game/_Core/Blueprint/GI_Game.GI_Game_C|GetShaktiHealth _asgi_game) 0))
    (CallFunction|GameOver)
    (else
      (for _array_element (Variables|Default|GetPlayers)
        (Variables|/Game/_Core/Blueprint/BP_BaseCharacter.BP_BaseCharacter_C|SetRoundNum (Variables|/Game/_Core/Blueprint/PC_PlayerController.PC_PlayerController_C|GetPossessed%20Pawn _array_element) (+ (Variables|/Game/_Core/Blueprint/BP_BaseCharacter.BP_BaseCharacter_C|GetRoundNum (Variables|/Game/_Core/Blueprint/PC_PlayerController.PC_PlayerController_C|GetPossessed%20Pawn _array_element)) 1))
        (if (Ability|HasAuthority _array_element)
          (CallFunction|Countdown)
          (Variables|Default|SetHostPlayer _array_element))))))

(event Custom|GameOver
  (Default|GameOver (Variables|/Game/_Core/Blueprint/PC_PlayerController.PC_PlayerController_C|GetPossessed%20Pawn (Variables|Default|GetHostPlayer)))
  (Utilities|FlowControl|Delay 1.0)
  (bind _asgi_game (Utilities|Casting|CastToGI_Game (Game|GetGameInstance)))
  (Default|StartGame _asgi_game)
  (for _array_element (Variables|Default|GetPlayers)
    (Default|ResetStats _array_element)))

(event EventBeginPlay)

(event EventTick
  (params (DeltaSeconds :type Float%20%28single-precision%29)))

(event EventHandleStartingNewPlayer
  (params (NewPlayer :type Player%20Controller%20Object%20Reference)))

(event EventPostLogin
  (params (NewPlayer :type Player%20Controller%20Object%20Reference))
  (bind _aspc_player_controller (Utilities|Casting|CastToPC_PlayerController NewPlayer))
  (Default|SetPlayerIndex _aspc_player_controller)
  (Default|StartGsme _aspc_player_controller)
  (Utilities|Array|Add (Variables|Default|GetPlayers) _aspc_player_controller)
  (bind _asbp_player_state (Utilities|Casting|CastToBP_PlayerState (Variables|/Script/Engine.Controller|GetPlayerState _aspc_player_controller)))
  (bind (_startposition _playernum) (CallFunction|GetPlayerStart NewPlayer _aspc_player_controller))
  (bind _returnvalue (Game|SpawnActorfromClass "/Game/_Core/Blueprint/BP_BaseCharacter.BP_BaseCharacter_C" (Transformation|GetActorTransform _startposition) "Undefined" 0 0))
  (Variables|/Game/_Core/Blueprint/BP_BaseCharacter.BP_BaseCharacter_C|SetPlayerNum _returnvalue _playernum)
  (Pawn|Possess _aspc_player_controller _returnvalue)
  (Default|SetPlayerRotation _returnvalue (.Rotation (Math|Transform|BreakTransform (Transformation|GetActorTransform _startposition))))
  (Variables|Default|SetRoundStarted false)
  (bind _asgi_game (Utilities|Casting|CastToGI_Game (Game|GetGameInstance)))
  (Default|StartGame _asgi_game)
  (if (== (Utilities|Array|Length (Variables|Default|GetPlayers)) 2)
    (CallFunction|StartCountdown)
    (for _array_element (Variables|Default|GetPlayers)
      (Default|SetPlayersName _array_element)
      (Default|ResetStats _array_element))))

(fn ConstructionScript)

(fn ChoosePlayerStart
  (params (Player :type Controller%20Object%20Reference)))

(fn GetPlayerStart
  (params (Player :type Controller%20Object%20Reference) (Controller :type PC%20Player%20Controller%20Object%20Reference))
  (bind _playerindex (Variables|/Game/_Core/Blueprint/PC_PlayerController.PC_PlayerController_C|GetPlayerIndex Controller))
  (bind _players (Variables|Default|GetPlayers))
  (bind _returnvalue (Utilities|String|ToString(Integer) _playerindex))
  (bind _output (Utilities|Array|Get(acopy) _players))
  (bind _returnvalue_2 (Class|GameModeBase|FindPlayerStart Player _returnvalue))
  (bind _playerindex_2 (Variables|/Game/_Core/Blueprint/PC_PlayerController.PC_PlayerController_C|GetPlayerIndex _output))
  (if (== (Utilities|Array|Length (Variables|Default|GetPlayers)) 1)
    (Utilities|IsValid _returnvalue_2
      (:Is%20Valid
        (return _returnvalue_2 (Variables|/Game/_Core/Blueprint/PC_PlayerController.PC_PlayerController_C|GetPlayerIndex Controller))))
    (elif (== _playerindex_2 0)
      (return (Class|GameModeBase|FindPlayerStart Player "1") 1)
      (elif (== _playerindex_2 1)
        (return (Class|GameModeBase|FindPlayerStart Player "0") 0)))))

(fn GetStartIndex
  (bind _asgi_game (Utilities|Casting|CastToGI_Game (Game|GetGameInstance)))
  (switch Utilities|FlowControl|Switch|SwitchonPlayerType (Variables|/Script/chakra_clash.EOSGameInstance|GetSelectedPlayer _asgi_game)
    (:Deva
      (return (- (Utilities|Array|Length (Variables|Default|GetPlayers)) 1)))))