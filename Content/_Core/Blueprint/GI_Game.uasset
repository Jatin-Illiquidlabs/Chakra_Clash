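; GI_Game is the game instance Blueprint that holds health and charge for two characters, Deva and Shakti.
; Separate events subtract damage from each health value and add to each charge, capping charge at a fixed maximum with no lower clamp.
; StartGame resets both characters to the default health and charge.
; Disconnected nodes for opening the gate_night level and destroying the session never run.
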(event Custom|UpdateDevaHealth
  (params (Damage :type Integer))
  (Variables|Default|SetDevaHealth (- (Variables|Default|GetDevaHealth) Damage)))

(event Custom|UpdateShaktiHealth
  (params (Damage :type Integer))
  (Variables|Default|SetShaktiHealth (- (Variables|Default|GetShaktiHealth) Damage)))

(event Custom|UpdateDevaCharge
  (params (ChangeAmount :type Integer))
  (bind _output_get (Variables|Default|SetDevaCharge (+ (Variables|Default|GetDevaCharge) ChangeAmount)))
  (if (>= _output_get 10)
    (Variables|Default|SetDevaCharge 10)))

(event Custom|UpdateShaktiCharge
  (params (ChangeAmount :type Integer))
  (bind _output_get (Variables|Default|SetShaktiCharge (+ (Variables|Default|GetShaktiCharge) ChangeAmount)))
  (if (>= _output_get 10)
    (Variables|Default|SetShaktiCharge 10)))

(event Custom|StartGame
  (bind _defaulthealth (Variables|Default|GetDefaultHealth))
  (bind _defaultcharge (Variables|Default|GetDefaultCharge))
  (Variables|Default|SetDevaHealth _defaulthealth)
  (Variables|Default|SetShaktiHealth _defaulthealth)
  (Variables|Default|SetDevaCharge _defaultcharge)
  (Variables|Default|SetShaktiCharge _defaultcharge))