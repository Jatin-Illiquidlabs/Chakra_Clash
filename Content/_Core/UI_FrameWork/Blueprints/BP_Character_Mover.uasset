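; Helper actor that positions and animates display characters at preset Player 1, Player 2, Character Select and far-away spots, apparently for UI screens.
; It tracks an active index into a character array and a current location chosen by slot.
; Switching character sends the mover itself to the far-away spot and teleports the new character to the current location.
; Separate functions reposition the active character or play looping animations, with idle played on slot changes.
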(event EventBeginPlay)

(event Collision|EventActorBeginOverlap
  (params (OtherActor :type Actor%20Object%20Reference)))

(event EventTick
  (params (DeltaSeconds :type Float%20%28single-precision%29)))

(fn ConstructionScript)

(fn ChangeActiveCharacter
  (params (Character :type Integer))
  (Transformation|SetActorLocation (Variables|Default|GetFaraway%20Loc) false true)
  (bind _output_get (Variables|Default|SetActive%20Character%20Index Character))
  (Transformation|SetActorLocation (Utilities|Array|Get(acopy) (Variables|Default|GetAll%20Characters) _output_get) (Variables|Default|GetCurrent%20Active%20Loc) false true))

(fn SetCurrentActiveLocation
  (params (Current%20Active%20Loc :type CharacterLocation_ENUM%20Enum :default "NewEnumerator14"))
  (Utilities|FlowControl|Sequence
    (:then_0
      (switch Utilities|FlowControl|Switch|SwitchonCharacterLocation_ENUM Current%20Active%20Loc
        (:NewEnumerator14
          (Variables|Default|SetCurrent%20Active%20Loc (Variables|Default|GetPlayer%201%20Location)))
        (:NewEnumerator15
          (Variables|Default|SetCurrent%20Active%20Loc (Variables|Default|GetPlayer%202%20Location)))
        (:NewEnumerator16
          (Variables|Default|SetCurrent%20Active%20Loc (Variables|Default|GetCharacter%20Select%20Location)))
        (:NewEnumerator17
          (Variables|Default|SetCurrent%20Active%20Loc (Variables|Default|GetFaraway%20Loc)))))
    (:then_1
      (CallFunction|ChangeActiveCharacterAnimation "/Game/Nodachi_Animset/Animation/Anim_idle.Anim_idle"))))

(fn ChangeActiveCharacterLocation
  (Transformation|SetActorLocation (Utilities|Array|Get(acopy) (Variables|Default|GetAll%20Characters) (Variables|Default|GetActive%20Character%20Index)) (Variables|Default|GetCurrent%20Active%20Loc) false false)
  (Development|PrintString "Changed actor location"))

(fn ChangeActiveCharacterAnimation
  (params (NewAnimToPlay :type Animation%20Asset%20Object%20Reference))
  (Components|Animation|PlayAnimation (Variables|/Script/Engine.Character|GetMesh (Utilities|Array|Get(acopy) (Variables|Default|GetAll%20Characters) (Variables|Default|GetActive%20Character%20Index))) NewAnimToPlay true))