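; BP_SpaceSkyBox is a space skybox actor whose brightness animates when play begins.
; The construction script applies M_Space to the static mesh.
; On BeginPlay, it replaces that with a dynamic instance of MI_Space, and the Brightness timeline drives the instance's Brightness scalar parameter on each update.
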(event EventBeginPlay
  (bind _returnvalue (Rendering|Material|CreateDynamicMaterialInstance "/Game/ScanlineVFX/Material/Level/MI_Space.MI_Space" "None" "None" :!class /Script/Engine.KismetMaterialLibrary))
  (Variables|Default|SetSpace _returnvalue)
  (Rendering|Material|SetMaterial (Variables|Default|GetStaticMesh) 0 (Variables|Default|GetSpace))
  (bind _newtrack_0 (Timeline|Brightness Play)
    (:Update
      (Rendering|Material|SetScalarParameterValue (Variables|Default|GetSpace) "Brightness" _newtrack_0 :!class /Script/Engine.MaterialInstanceDynamic))))

(fn ConstructionScript
  (Rendering|Material|SetMaterial (Variables|Default|GetStaticMesh) 0 "/Game/ScanlineVFX/Material/Level/M_Space.M_Space"))