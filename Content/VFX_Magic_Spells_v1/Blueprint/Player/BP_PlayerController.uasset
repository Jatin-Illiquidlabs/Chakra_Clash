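; Player controller for a VFX spell showcase that binds twenty keys to spells from DT_Spells through a shared Cast macro.
; Holding a key freezes look input and moves a target decal under the cursor; releasing spawns the effect at the cursor hit (Boost).
; Shift instead spawns it immediately at the pawn's feet (Nova), while Alt attaches it to the pawn (Emanation), taking priority over Shift.
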(event EventTick
  (params (DeltaSeconds :type Float%20%28single-precision%29))
  (if (Utilities|Name|NotEqual(Name) (Variables|Default|GetEnableAreaIndex) "0")
    (Transformation|SetWorldLocation (Variables|Default|GetTargetArea) (.Location (Collision|BreakHitResult (.HitResult (Game|Player|GetHitResultUnderCursorbyChannel "TraceTypeQuery1" true)))) true false)))

(event Input|AxisEvents|InputAxisLookUp
  (params (AxisValue :type Float%20%28single-precision%29))
  (if (not (Utilities|Name|NotEqual(Name) (Variables|Default|GetEnableAreaIndex) "0"))
    (Class|PlayerController|AddPitchInput AxisValue)))

(event Input|AxisEvents|InputAxisTurn
  (params (AxisValue :type Float%20%28single-precision%29))
  (if (not (Utilities|Name|NotEqual(Name) (Variables|Default|GetEnableAreaIndex) "0"))
    (Class|PlayerController|AddYawInput AxisValue)))

(event Input|KeyboardEvents|LeftShift
  (params (Key :type Key%20Structure))
  (:Pressed
    (Variables|Default|SetShift true))
  (:Released
    (Variables|Default|SetShift false)))

(event Input|KeyboardEvents|1
  (params (Key :type Key%20Structure))
  (:Pressed
    (Utilities|Cast "1" "1.000000,250.000000,250.000000" :!label _label))
  (:Released
    (goto _label Released)))

(event Input|KeyboardEvents|7
  (params (Key :type Key%20Structure))
  (:Pressed
    (Utilities|Cast "7" "1.000000,150.000000,150.000000" :!label _label))
  (:Released
    (goto _label Released)))

(event Input|KeyboardEvents|8
  (params (Key :type Key%20Structure))
  (:Pressed
    (Utilities|Cast "8" "1.000000,225.000000,225.000000" :!label _label))
  (:Released
    (goto _label Released)))

(event Input|KeyboardEvents|9
  (params (Key :type Key%20Structure))
  (bind _returnvalue (Pawn|GetControlledPawn))
  (bind (_ascharacter _bsuccess) (Utilities|Casting|CastToCharacter _returnvalue))
  (:Pressed
    (Utilities|Cast "9" (Math|Vector|MakeVector (select _bsuccess (Components|Capsule|GetScaledCapsuleHalfHeight (Variables|/Script/Engine.Character|GetCapsuleComponent _ascharacter)) 5e+01) 125.0 125.0) :!label _label))
  (:Released
    (goto _label Released)))

(event Input|KeyboardEvents|0
  (params (Key :type Key%20Structure))
  (:Pressed
    (Utilities|Cast "10" "1.000000,200.000000,200.000000" :!label _label))
  (:Released
    (goto _label Released)))

(event Input|KeyboardEvents|C
  (params (Key :type Key%20Structure))
  (bind _returnvalue (Pawn|GetControlledPawn))
  (bind (_ascharacter _bsuccess) (Utilities|Casting|CastToCharacter _returnvalue))
  (:Pressed
    (Utilities|Cast "13" (Math|Vector|MakeVector (select _bsuccess (Components|Capsule|GetScaledCapsuleHalfHeight (Variables|/Script/Engine.Character|GetCapsuleComponent _ascharacter)) 5e+01) 125.0 125.0) :!label _label))
  (:Released
    (goto _label Released)))

(event Input|KeyboardEvents|V
  (params (Key :type Key%20Structure))
  (:Pressed
    (Utilities|Cast "14" "1.000000,350.000000,350.000000" :!label _label))
  (:Released
    (goto _label Released)))

(event Input|KeyboardEvents|B
  (params (Key :type Key%20Structure))
  (:Pressed
    (Utilities|Cast "15" "1.000000,235.000000,235.000000" :!label _label))
  (:Released
    (goto _label Released)))

(event Input|KeyboardEvents|N
  (params (Key :type Key%20Structure))
  (:Pressed
    (Utilities|Cast "16" "1.000000,335.000000,335.000000" :!label _label))
  (:Released
    (goto _label Released)))

(event Input|KeyboardEvents|M
  (params (Key :type Key%20Structure))
  (:Pressed
    (Utilities|Cast "17" "1.000000,350.000000,350.000000" :!label _label))
  (:Released
    (goto _label Released)))

(event Input|KeyboardEvents|F
  (params (Key :type Key%20Structure))
  (:Pressed
    (Utilities|Cast "18" "1.000000,175.000000,175.000000" :!label _label))
  (:Released
    (goto _label Released)))

(event Input|KeyboardEvents|Z
  (params (Key :type Key%20Structure))
  (:Pressed
    (Utilities|Cast "11" "1.000000,150.000000,150.000000" :!label _label))
  (:Released
    (goto _label Released)))

(event Input|KeyboardEvents|G
  (params (Key :type Key%20Structure))
  (:Pressed
    (Utilities|Cast "19" "1.000000,250.000000,250.000000" :!label _label))
  (:Released
    (goto _label Released)))

(event Input|KeyboardEvents|H
  (params (Key :type Key%20Structure))
  (:Pressed
    (Utilities|Cast "20" "1.000000,210.000000,210.000000" :!label _label))
  (:Released
    (goto _label Released)))

(event Input|KeyboardEvents|3
  (params (Key :type Key%20Structure))
  (:Pressed
    (Utilities|Cast "3" "1.000000,335.000000,335.000000" :!label _label))
  (:Released
    (goto _label Released)))

(event Input|KeyboardEvents|2
  (params (Key :type Key%20Structure))
  (bind _returnvalue (Pawn|GetControlledPawn))
  (bind (_ascharacter _bsuccess) (Utilities|Casting|CastToCharacter _returnvalue))
  (:Pressed
    (Utilities|Cast "2" (Math|Vector|MakeVector (select _bsuccess (Components|Capsule|GetScaledCapsuleHalfHeight (Variables|/Script/Engine.Character|GetCapsuleComponent _ascharacter)) 5e+01) 125.0 125.0) :!label _label))
  (:Released
    (goto _label Released)))

(event Input|KeyboardEvents|X
  (params (Key :type Key%20Structure))
  (:Pressed
    (Utilities|Cast "12" "1.000000,325.000000,325.000000" :!label _label))
  (:Released
    (goto _label Released)))

(event Input|KeyboardEvents|LeftAlt
  (params (Key :type Key%20Structure))
  (:Pressed
    (Variables|Default|SetAlt true))
  (:Released
    (Variables|Default|SetAlt false)))

(event Input|KeyboardEvents|4
  (params (Key :type Key%20Structure))
  (:Pressed
    (Utilities|Cast "4" "1.000000,300.000000,300.000000" :!label _label))
  (:Released
    (goto _label Released)))

(event Input|KeyboardEvents|5
  (params (Key :type Key%20Structure))
  (:Pressed
    (Utilities|Cast "5" "1.000000,500.000000,500.000000" :!label _label))
  (:Released
    (goto _label Released)))

(event Input|KeyboardEvents|6
  (params (Key :type Key%20Structure))
  (bind _returnvalue (Pawn|GetControlledPawn))
  (bind (_ascharacter _bsuccess) (Utilities|Casting|CastToCharacter _returnvalue))
  (:Pressed
    (Utilities|Cast "6" (Math|Vector|MakeVector (select _bsuccess (Components|Capsule|GetScaledCapsuleHalfHeight (Variables|/Script/Engine.Character|GetCapsuleComponent _ascharacter)) 5e+01) 125.0 125.0) :!label _label))
  (:Released
    (goto _label Released)))

(fn ConstructionScript)

(fn Boost
  (params (SpellIndex :type Name) (LocationZ :type Float%20%28double-precision%29))
  (bind _hitresult (Game|Player|GetHitResultUnderCursorbyChannel "TraceTypeQuery1" true))
  (bind _location (Collision|BreakHitResult _hitresult))
  (bind _returnvalue (Utilities|GetDataTableRow "/Game/VFX_Magic_Spells_v1/Blueprint/Player/DT_Spells.DT_Spells" SpellIndex)
    (:then
      (Niagara|SpawnSystematLocation (.vfx _returnvalue) (Math|Vector|MakeVector (.x _location) (.y _location) (+ LocationZ (.z _location))) (Math|Rotator|MakeRotator 0.0 0.0 (.yaw (Pawn|GetControlRotation :!class /Script/Engine.Controller))))
      (Variables|Default|SetEnableAreaIndex "0"))))

(fn Nova
  (params (SpellIndex :type Name) (LocationZ :type Float%20%28double-precision%29))
  (bind _returnvalue (Pawn|GetControlledPawn))
  (bind _returnvalue_2 (Utilities|GetDataTableRow "/Game/VFX_Magic_Spells_v1/Blueprint/Player/DT_Spells.DT_Spells" SpellIndex)
    (:then
      (Niagara|SpawnSystematLocation (.vfx _returnvalue_2) (- (Transformation|GetActorLocation _returnvalue) (Math|Vector|MakeVector 0.0 0.0 (- (Components|Capsule|GetScaledCapsuleHalfHeight (Variables|/Script/Engine.Character|GetCapsuleComponent (.AsCharacter (Utilities|Casting|CastToCharacter _returnvalue)))) LocationZ)))))))

(fn Emanation
  (params (SpellIndex :type Name) (LocationZ :type Float%20%28double-precision%29))
  (bind _returnvalue (Pawn|GetControlledPawn))
  (bind _returnvalue_2 (Utilities|GetDataTableRow "/Game/VFX_Magic_Spells_v1/Blueprint/Player/DT_Spells.DT_Spells" SpellIndex)
    (:then
      (Niagara|SpawnSystemAttached (.vfx _returnvalue_2) (Variables|/Script/Engine.Actor|GetRootComponent _returnvalue) "None" (Math|Vector|MakeVector 0.0 0.0 (+ LocationZ (* (Components|Capsule|GetScaledCapsuleHalfHeight (Variables|/Script/Engine.Character|GetCapsuleComponent (.AsCharacter (Utilities|Casting|CastToCharacter _returnvalue)))) -1.0))) "0, 0, 0" "KeepRelativeOffset" true))))

(fn ShowArea
  (params (EnableAreaIndex :type Name) (DecalSize :type Vector))
  (bind (_sizex _sizey) (HUD|GetViewportSize))
  (bind _returnvalue (/ (Utilities|Struct|MakeIntPoint _sizex _sizey) 2))
  (Variables|Default|SetEnableAreaIndex EnableAreaIndex)
  (Class|PlayerController|SetMouseLocation (.x _returnvalue) (.y _returnvalue))
  (bind _returnvalue_2 (Rendering|Decal|SpawnDecalatLocation "/Game/VFX_Magic_Spells_v1/Demo/Materials/Mi_Target.Mi_Target" (Math|Vector|MakeVector (Variables|Default|GetDecalHeight) (.y DecalSize) (.z DecalSize)) (.Location (Collision|BreakHitResult (.HitResult (Game|Player|GetHitResultUnderCursorbyChannel "TraceTypeQuery1" true)))) (Math|Rotator|MakeRotator 0.0 -9e+01 (.yaw (Pawn|GetControlRotation :!class /Script/Engine.Controller))) 0.0))
  (Variables|Default|SetTargetArea _returnvalue_2))

(fn HideArea
  (Variables|Default|SetEnableAreaIndex "0")
  (Components|DestroyComponent (Variables|Default|GetTargetArea))
  (Variables|Default|SetTargetArea 0))