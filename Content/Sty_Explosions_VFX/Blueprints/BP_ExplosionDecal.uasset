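; Explosion decal actor that applies a randomly rolled decal, animates it in and out, then destroys itself.
; BeginPlay creates a dynamic material instance whose Erosion parameter runs through an optional implosion fade-in, a delay and a fade timeline.
; An optional Emissive pass uses the same fade-in time, then plays its own timeline without the delay.
; The construction script sets the decal component's fade-out to match the erosion timing and destroy the owner.
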(event Custom|EmissiveErosion
  (if (> (Variables|Default|GetImplosionFadeIn) 0.0)
    (Components|Timeline|SetPlayRate (Variables|Default|GetTimeline_EmissiveFadeIn) (/ 1.0 (Variables|Default|GetImplosionFadeIn)))
    (bind _erosion (Timeline|Timeline_EmissiveFadeIn PlayFromStart)
      (:Update
        (Rendering|Material|SetScalarParameterValue (Variables|Default|GetDynamicMat) "Emissive" _erosion :!class /Script/Engine.MaterialInstanceDynamic))
      (:Finished
        (Components|Timeline|SetPlayRate (Variables|Default|GetTimeline_Emissive) (/ 1.0 (Variables|Default|GetEmissiveDuration)) :!label _label)
        (bind _erosion_2 (Timeline|Timeline_Emissive PlayFromStart)
          (:Update
            (Rendering|Material|SetScalarParameterValue (Variables|Default|GetDynamicMat) "Emissive" _erosion_2 :!class /Script/Engine.MaterialInstanceDynamic)))))
    (else
      (goto _label))))

(event Custom|Erosion
  (if (> (Variables|Default|GetImplosionFadeIn) 0.0)
    (Components|Timeline|SetPlayRate (Variables|Default|GetTimeline_ErosionFadeIn) (/ 1.0 (Variables|Default|GetImplosionFadeIn)))
    (bind _erosion (Timeline|Timeline_ErosionFadeIn PlayFromStart)
      (:Update
        (Rendering|Material|SetScalarParameterValue (Variables|Default|GetDynamicMat) "Erosion" _erosion :!class /Script/Engine.MaterialInstanceDynamic))
      (:Finished
        (Utilities|FlowControl|Delay (Variables|Default|GetStart%20Delay) :!label _label)
        (Components|Timeline|SetPlayRate (Variables|Default|GetErosion_Timeline) (/ 1.0 (Variables|Default|GetFadeDuration)))
        (bind _erosion_2 (Timeline|Erosion_Timeline PlayFromStart)
          (:Update
            (Rendering|Material|SetScalarParameterValue (Variables|Default|GetDynamicMat) "Erosion" _erosion_2 :!class /Script/Engine.MaterialInstanceDynamic)))))
    (else
      (Rendering|Material|SetScalarParameterValue (Variables|Default|GetDynamicMat) "Erosion" 1.0 :!class /Script/Engine.MaterialInstanceDynamic)
      (goto _label))))

(event EventBeginPlay
  (bind _decal (Variables|Decal|GetDecal))
  (Transformation|AddActorLocalRotation (Math|Rotator|MakeRotator (Math|Random|RandomFloatinRange 0.0 3.6e+02) 0.0 0.0) false false)
  (Rendering|Components|Decal|SetDecalMaterial _decal (Variables|Default|GetDecalMaterial))
  (bind _returnvalue (Rendering|Material|CreateDynamicMaterialInstance _decal :!class /Script/Engine.DecalComponent))
  (Variables|Default|SetDynamicMat _returnvalue)
  (CallFunction|Erosion)
  (if (Variables|Default|GetEmissive)
    (CallFunction|EmissiveErosion)))

(fn ConstructionScript
  (Rendering|Components|Decal|SetFadeOut (Variables|Decal|GetDecal) (+ (Variables|Default|GetStart%20Delay) (Variables|Default|GetImplosionFadeIn)) (Variables|Default|GetFadeDuration) true))